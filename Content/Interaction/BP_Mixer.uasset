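; BP_Mixer is an interactable that combines held ingredients into vaccines or waste.
; A server event flips InteractToggle, whose OnRep advances the tutorial and runs Interact on the first character found to add an ingredient, empty the mixer or collect a vaccine.
; Up to three distinct ingredients show as materials and widget text.
; Mix, not called within this Blueprint, matches hardcoded recipes and otherwise yields waste.
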(event Custom|InteractOnServer
  (Variables|Default|SetInteractToggle (not (Variables|Default|GetInteractToggle))))

(event EventBeginPlay
  (Development|ExecuteConsoleCommand "ENABLEALLSCREENMESSAGES" 0)
  (bind _asbp_interaction_area (Utilities|Casting|CastToBP_InteractionArea (Variables|/Script/Engine.ChildActorComponent|GetChildActor (Variables|Default|GetChildActor))))
  (Variables|/Game/Interaction/InteractionArea/BP_InteractionArea.BP_InteractionArea_C|SetObjectID _asbp_interaction_area (Variables|Default|GetObjectID)))

(event Collision|EventActorBeginOverlap
  (params (OtherActor :type Actor%20Object%20Reference)))

(event EventTick
  (params (DeltaSeconds :type Float%20%28single-precision%29)))

(event EventInterfaceToggleFocus
  (params (Focus :type Boolean))
  (Rendering|SetRenderCustomDepth (Variables|Default|GetCube) Focus))

(event EventInterfaceInteract
  (CallFunction|InteractonServer))

(fn ConstructionScript)

(fn OnRepInteractToggle
  (bind _asbp_first_person_game_mode (Utilities|Casting|CastToBP_FirstPersonGameMode (Game|GetGameMode)))
  (if (Variables|/Game/FirstPerson/Blueprints/BP_FirstPersonGameMode.BP_FirstPersonGameMode_C|GetTutorialMode _asbp_first_person_game_mode)
    (bind _output_get (Variables|Default|SetIngredient (+ (Variables|Default|GetIngredient) 1)))
    (if (== _output_get 2)
      (Default|TutorialTimer _asbp_first_person_game_mode 1.0)))
  (bind _outactors (Actor|GetAllActorsOfClass "/Game/FirstPerson/Blueprints/BP_FirstPersonCharacter.BP_FirstPersonCharacter_C"))
  (Components|StaticMesh|SetStaticMesh (Variables|/Game/FirstPerson/Blueprints/BP_FirstPersonCharacter.BP_FirstPersonCharacter_C|GetItem (Utilities|Array|Get(acopy) _outactors)) (Variables|Default|GetMesh))
  (CallFunction|Interact (Variables|/Game/FirstPerson/Blueprints/BP_FirstPersonCharacter.BP_FirstPersonCharacter_C|GetIngredientHolding (Utilities|Array|Get(acopy) _outactors)))
  (Audio|SpawnSound2D "/Game/Assets/Audio/place-glass-object-81857.place-glass-object-81857" 1.0 1.0 2.0 0))

(fn Interact
  (params (In :type String))
  (if (Variables|Default|GetContainsWaste)
    (Variables|Default|SetContainsWaste false :!label _label)
    ;[1 0.1855 0.1557] Set widget text
    (bind _output_get (Variables|Default|SetTemp "None"))
    (bind _aswb_interaction (Utilities|Casting|CastToWB_Interaction (UserInterface|GetWidget (Variables|Default|GetWidget))))
    (Variables|/Game/Interaction/WB_Interaction.WB_Interaction_C|SetText _aswb_interaction _output_get)
    (elif (Variables|Default|GetContainsVaccine)
      ;[1 0.1855 0.1557] Pickup vaccine
      (bind _outactors (Actor|GetAllActorsOfClass "/Game/FirstPerson/Blueprints/BP_FirstPersonCharacter.BP_FirstPersonCharacter_C"))
      (if (Variables|/Game/FirstPerson/Blueprints/BP_FirstPersonCharacter.BP_FirstPersonCharacter_C|GetIsHolding (Utilities|Array|Get(acopy) _outactors))
        (Development|PrintString "Can't pick up while holding")
        (else
          (Variables|/Game/FirstPerson/Blueprints/BP_FirstPersonCharacter.BP_FirstPersonCharacter_C|SetHoldingVaccine (Utilities|Array|Get(acopy) _outactors) true)
          (Variables|/Game/FirstPerson/Blueprints/BP_FirstPersonCharacter.BP_FirstPersonCharacter_C|SetVaccine (Utilities|Array|Get(acopy) _outactors) (Variables|Default|GetVaccine))
          (Components|StaticMesh|SetStaticMesh (Variables|/Game/FirstPerson/Blueprints/BP_FirstPersonCharacter.BP_FirstPersonCharacter_C|GetItem (Utilities|Array|Get(acopy) _outactors)) "/Game/Assets/Models/Ingredientflask_Carben.Ingredientflask_Carben")
          (Variables|Default|SetContainsVaccine false)
          (bind _outactors_2 (Actor|GetAllActorsOfClass "/Game/Interaction/BP_ShipmentBox.BP_ShipmentBox_C"))
          (Default|ToggleInteractable (Utilities|Array|Get(acopy) _outactors_2) true)
          (Rendering|Material|SetMaterial (Variables|Default|GetCube) 0 "/Game/Assets/Materials/InvisibleIngredient.InvisibleIngredient")
          (Rendering|Material|SetMaterial (Variables|Default|GetCube) 1 "/Game/Assets/Materials/InvisibleIngredient.InvisibleIngredient")
          (Rendering|Material|SetMaterial (Variables|Default|GetCube) 2 "/Game/Assets/Materials/InvisibleIngredient.InvisibleIngredient")
          (goto _label)))
      (else
        ;[1 0.1855 0.1557] Determine between adding ingredient or emptying
        (bind _outactors_3 (Actor|GetAllActorsOfClass "/Game/FirstPerson/Blueprints/BP_FirstPersonCharacter.BP_FirstPersonCharacter_C"))
        (if (Variables|/Game/FirstPerson/Blueprints/BP_FirstPersonCharacter.BP_FirstPersonCharacter_C|GetIsHolding (Utilities|Array|Get(acopy) _outactors_3))
          ;[1 0.1855 0.1557] Exit if mixer already full
          (if (not (== (Utilities|Array|Length (Variables|Default|GetIngredients)) 3))
            (bind _outactors_4 (Actor|GetAllActorsOfClass "/Game/FirstPerson/Blueprints/BP_FirstPersonCharacter.BP_FirstPersonCharacter_C"))
            (Variables|/Game/FirstPerson/Blueprints/BP_FirstPersonCharacter.BP_FirstPersonCharacter_C|SetIsHolding (Utilities|Array|Get(acopy) _outactors_4) false)
            ;[1 0.1855 0.1557] Check each ingredient in mixer for copies
            (bind (_array_element _array_index) (Utilities|Array|ForEachLoopwithBreak (Variables|Default|GetIngredients))
              (:LoopBody
                (if (Utilities|Enum|Equal(Enum) (.Name (Utilities|Struct|BreakIngredient _array_element)) In)
                  ;[1 0.1855 0.1557] Increment quantity if already in mixer
                  (LocalVariables|SetInArray true)
                  (Utilities|Array|SetArrayElem (Variables|Default|GetIngredients) _array_index (Utilities|Struct|MakeIngredient (.Name (Utilities|Struct|BreakIngredient _array_element)) (+ (.Quantity (Utilities|Struct|BreakIngredient _array_element)) 1) 0 0))
                  (Development|PrintString (Utilities|String|ToString(Integer) (.Quantity (Utilities|Struct|BreakIngredient _array_element))))
                  (Development|PrintString "Added")
                  (Variables|Default|SetTemp "" :!label _label_2)
                  ;[1 0.1855 0.1557] Loop through each ingredient in mixer
                  (for (_array_element_2 _array_index_2) (Variables|Default|GetIngredients)
                    (if (== _array_index_2 0)
                      ;[1 0.1855 0.1557] Add text for ingredient #1
                      (Variables|Default|SetTemp (Utilities|String|Append (Variables|Default|GetTemp) (Utilities|String|Append (Utilities|String|Append (.Name (Utilities|Struct|BreakIngredient _array_element_2)) (Utilities|String|MakeLiteralString " x")) (Utilities|String|ToString(Integer) (.Quantity (Utilities|Struct|BreakIngredient _array_element_2))))))
                      (else
                        ;[1 0.1855 0.1557] Add text for ingredients #2/3
                        (bind _output_get_2 (Variables|Default|SetTemp (Utilities|String|Append (Variables|Default|GetTemp) (Utilities|String|Append (Utilities|String|Append (Utilities|String|Append (Utilities|String|MakeLiteralString " 
") (.Name (Utilities|Struct|BreakIngredient _array_element_2))) (Utilities|String|MakeLiteralString " x")) (Utilities|String|ToString(Integer) (.Quantity (Utilities|Struct|BreakIngredient _array_element_2)))))))))
                    ;[1 0.1855 0.1557] Set widget text
                    (bind _aswb_interaction_2 (Utilities|Casting|CastToWB_Interaction (UserInterface|GetWidget (Variables|Default|GetWidget))))
                    (Variables|/Game/Interaction/WB_Interaction.WB_Interaction_C|SetText _aswb_interaction_2 _output_get_2))))
              (:Completed
                ;[1 0.1855 0.1557] Add ingredient if not in mixer
                (if (not (LocalVariables|GetInArray))
                  (bind _returnvalue (Utilities|Array|Add (Variables|Default|GetIngredients) (Utilities|Struct|MakeIngredient In 1 0 0)))
                  (if (== _returnvalue 0)
                    (switch string In
                      (:Carben
                        (Rendering|Material|SetMaterial (Variables|Default|GetCube) 0 "/Game/Assets/Materials/Carben.Carben")
                        (goto _label_2))
                      (:Magnesien
                        (Rendering|Material|SetMaterial (Variables|Default|GetCube) 0 "/Game/Assets/Materials/Magnesien.Magnesien")
                        (goto _label_2))
                      (:Sodien
                        (Rendering|Material|SetMaterial (Variables|Default|GetCube) 0 "/Game/Assets/Materials/Sodien.Sodien")
                        (goto _label_2))
                      (:Tungen
                        (Rendering|Material|SetMaterial (Variables|Default|GetCube) 0 "/Game/Assets/Materials/Tungen.Tungen")
                        (goto _label_2))
                      (:Heldon
                        (Rendering|Material|SetMaterial (Variables|Default|GetCube) 0 "/Game/Assets/Materials/Heldon.Heldon")
                        (goto _label_2))
                      (:Hydon
                        (Rendering|Material|SetMaterial (Variables|Default|GetCube) 0 "/Game/Assets/Materials/Hydon.Hydon")
                        (goto _label_2))
                      (:Fluoren
                        (Rendering|Material|SetMaterial (Variables|Default|GetCube) 0 "/Game/Assets/Materials/Fluoren.Fluoren")
                        (goto _label_2))
                      (:Oxyden
                        (Rendering|Material|SetMaterial (Variables|Default|GetCube) 0 "/Game/Assets/Materials/Oxyden.Oxyden")
                        (goto _label_2)))
                    (elif (== _returnvalue 2)
                      (switch string In
                        (:Carben
                          (Rendering|Material|SetMaterial (Variables|Default|GetCube) 1 "/Game/Assets/Materials/Carben.Carben")
                          (goto _label_2))
                        (:Magnesien
                          (Rendering|Material|SetMaterial (Variables|Default|GetCube) 1 "/Game/Assets/Materials/Magnesien.Magnesien")
                          (goto _label_2))
                        (:Sodien
                          (Rendering|Material|SetMaterial (Variables|Default|GetCube) 1 "/Game/Assets/Materials/Sodien.Sodien")
                          (goto _label_2))
                        (:Tungen
                          (Rendering|Material|SetMaterial (Variables|Default|GetCube) 1 "/Game/Assets/Materials/Tungen.Tungen")
                          (goto _label_2))
                        (:Heldon
                          (Rendering|Material|SetMaterial (Variables|Default|GetCube) 1 "/Game/Assets/Materials/Heldon.Heldon")
                          (goto _label_2))
                        (:Hydon
                          (Rendering|Material|SetMaterial (Variables|Default|GetCube) 1 "/Game/Assets/Materials/Hydon.Hydon")
                          (goto _label_2))
                        (:Fluoren
                          (Rendering|Material|SetMaterial (Variables|Default|GetCube) 1 "/Game/Assets/Materials/Fluoren.Fluoren")
                          (goto _label_2))
                        (:Oxyden
                          (Rendering|Material|SetMaterial (Variables|Default|GetCube) 1 "/Game/Assets/Materials/Oxyden.Oxyden")
                          (goto _label_2)))
                      (elif (== _returnvalue 1)
                        (switch string In
                          (:Carben
                            (Rendering|Material|SetMaterial (Variables|Default|GetCube) 2 "/Game/Assets/Materials/Carben.Carben")
                            (goto _label_2))
                          (:Magnesien
                            (Rendering|Material|SetMaterial (Variables|Default|GetCube) 2 "/Game/Assets/Materials/Magnesien.Magnesien")
                            (goto _label_2))
                          (:Sodien
                            (Rendering|Material|SetMaterial (Variables|Default|GetCube) 2 "/Game/Assets/Materials/Sodien.Sodien")
                            (goto _label_2))
                          (:Tungen
                            (Rendering|Material|SetMaterial (Variables|Default|GetCube) 2 "/Game/Assets/Materials/Tungen.Tungen")
                            (goto _label_2))
                          (:Heldon
                            (Rendering|Material|SetMaterial (Variables|Default|GetCube) 2 "/Game/Assets/Materials/Heldon.Heldon")
                            (goto _label_2))
                          (:Hydon
                            (Rendering|Material|SetMaterial (Variables|Default|GetCube) 2 "/Game/Assets/Materials/Hydon.Hydon")
                            (goto _label_2))
                          (:Fluoren
                            (Rendering|Material|SetMaterial (Variables|Default|GetCube) 2 "/Game/Assets/Materials/Fluoren.Fluoren")
                            (goto _label_2))
                          (:Oxyden
                            (Rendering|Material|SetMaterial (Variables|Default|GetCube) 2 "/Game/Assets/Materials/Oxyden.Oxyden")
                            (goto _label_2))))))))))
          (else
            (Development|PrintString "false")
            ;[1 0.1855 0.1557] Empty Mixer (Nothing in Hand)
            (Utilities|Array|Clear (Variables|Default|GetIngredients))
            (Rendering|Material|SetMaterial (Variables|Default|GetCube) 0 "/Game/Assets/Materials/InvisibleIngredient.InvisibleIngredient")
            (Rendering|Material|SetMaterial (Variables|Default|GetCube) 1 "/Game/Assets/Materials/InvisibleIngredient.InvisibleIngredient")
            (Rendering|Material|SetMaterial (Variables|Default|GetCube) 2 "/Game/Assets/Materials/InvisibleIngredient.InvisibleIngredient")
            (Variables|Default|SetContainsWaste false)
            (Variables|Default|SetTemp "None")
            (bind _aswb_interaction_3 (Utilities|Casting|CastToWB_Interaction (UserInterface|GetWidget (Variables|Default|GetWidget))))
            (Variables|/Game/Interaction/WB_Interaction.WB_Interaction_C|SetText _aswb_interaction_3 _output_get_2)))))))

(fn Mix
  (if (or (Variables|Default|GetContainsVaccine) (Variables|Default|GetContainsWaste))
    (Development|PrintString "Mixer contains unmixable items")
    (elif (== (Utilities|Array|Length (Variables|Default|GetIngredients)) 0)
      (Development|PrintString "Mixer is Empty")
      (else
        (Development|PrintString "Mixing")
        ;[1 1 1] Besmuth
        (if (and (and (and (Utilities|Array|ContainsItem (Variables|Default|GetIngredients) (Utilities|Struct|MakeIngredient "Carben" 1 0 0)) (Utilities|Array|ContainsItem (Variables|Default|GetIngredients) (Utilities|Struct|MakeIngredient "Sodien" 1 0 0))) (Utilities|Array|ContainsItem (Variables|Default|GetIngredients) (Utilities|Struct|MakeIngredient "Heldon" 1 0 0))) (== (Utilities|Array|Length (Variables|Default|GetIngredients)) 3))
          (Variables|Default|SetVaccine "Besmuth")
          (Variables|Default|SetContainsVaccine true)
          (else
            ;[1 1 1] Ibrofen
            (if (and (and (and (Utilities|Array|ContainsItem (Variables|Default|GetIngredients) (Utilities|Struct|MakeIngredient "Sodien" 1 0 0)) (Utilities|Array|ContainsItem (Variables|Default|GetIngredients) (Utilities|Struct|MakeIngredient "Fluoren" 1 0 0))) (Utilities|Array|ContainsItem (Variables|Default|GetIngredients) (Utilities|Struct|MakeIngredient "Heldon" 1 0 0))) (== (Utilities|Array|Length (Variables|Default|GetIngredients)) 3))
              (Variables|Default|SetVaccine "Ibrofen")
              (Variables|Default|SetContainsVaccine true)
              (else
                ;[1 1 1] Adfil
                (if (and (and (and (Utilities|Array|ContainsItem (Variables|Default|GetIngredients) (Utilities|Struct|MakeIngredient "Magnesien" 1 0 0)) (Utilities|Array|ContainsItem (Variables|Default|GetIngredients) (Utilities|Struct|MakeIngredient "Fluoren" 1 0 0))) (Utilities|Array|ContainsItem (Variables|Default|GetIngredients) (Utilities|Struct|MakeIngredient "Hydon" 1 0 0))) (== (Utilities|Array|Length (Variables|Default|GetIngredients)) 3))
                  (Variables|Default|SetVaccine "Adfil")
                  (Variables|Default|SetContainsVaccine true)
                  (else
                    ;[1 1 1] Fanedrill
                    (if (and (and (and (Utilities|Array|ContainsItem (Variables|Default|GetIngredients) (Utilities|Struct|MakeIngredient "Tungen" 1 0 0)) (Utilities|Array|ContainsItem (Variables|Default|GetIngredients) (Utilities|Struct|MakeIngredient "Hydon" 1 0 0))) (Utilities|Array|ContainsItem (Variables|Default|GetIngredients) (Utilities|Struct|MakeIngredient "Oxyden" 1 0 0))) (== (Utilities|Array|Length (Variables|Default|GetIngredients)) 3))
                      (Variables|Default|SetVaccine "Fanedrill")
                      (Variables|Default|SetContainsVaccine true)
                      (else
                        ;[1 1 1] Galenol
                        (if (and (and (Utilities|Array|ContainsItem (Variables|Default|GetIngredients) (Utilities|Struct|MakeIngredient "Heldon" 1 0 0)) (Utilities|Array|ContainsItem (Variables|Default|GetIngredients) (Utilities|Struct|MakeIngredient "Oxyden" 1 0 0))) (== (Utilities|Array|Length (Variables|Default|GetIngredients)) 2))
                          (Variables|Default|SetVaccine "Galenol")
                          (Variables|Default|SetContainsVaccine true)
                          (else
                            ;[1 1 1] Galenol
                            (if (and (and (Utilities|Array|ContainsItem (Variables|Default|GetIngredients) (Utilities|Struct|MakeIngredient "Hydon" 1 0 0)) (Utilities|Array|ContainsItem (Variables|Default|GetIngredients) (Utilities|Struct|MakeIngredient "Oxyden" 1 0 0))) (== (Utilities|Array|Length (Variables|Default|GetIngredients)) 2))
                              (Variables|Default|SetVaccine "Galenol")
                              (Variables|Default|SetContainsVaccine true)
                              (else
                                (Variables|Default|SetVaccine "Waste")
                                (Variables|Default|SetContainsWaste true)))))))))))))
        (bind _aswb_interaction (Utilities|Casting|CastToWB_Interaction (UserInterface|GetWidget (Variables|Default|GetWidget))))
        (bind _output_get (Variables|Default|SetTemp (Variables|Default|GetVaccine)))
        (Variables|/Game/Interaction/WB_Interaction.WB_Interaction_C|SetText _aswb_interaction _output_get)
        (Utilities|Array|Clear (Variables|Default|GetIngredients))
        (if (not (Variables|Default|GetContainsWaste))
          (Audio|SpawnSound2D "/Game/Assets/Audio/tiny-splash-83778.tiny-splash-83778" 1.0 1.0 0.0 0))))))

(fn GetInteractionWidgetRef
  (bind _aswb_interaction (Utilities|Casting|CastToWB_Interaction (UserInterface|GetWidget (Variables|Default|GetWidget))))
  (Variables|/Game/Interaction/WB_Interaction.WB_Interaction_C|SetText _aswb_interaction (Variables|Default|GetTemp))
  (Default|EditSizeBox _aswb_interaction 3e+02)
  (return (Variables|Default|GetWidget)))