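; Interactable computer actor that opens a shop screen (W_Shop), seeded on BeginPlay with a few random patient entries.
; Interface events highlight the cube via custom depth and flip InteractToggle through InteractOnServer.
; Its OnRep switches light, UI, cursor and first character's movement lock, but only powers on, with sound, during game-mode tutorial, advancing its step.
; KeyPressOff forces the screen closed, and a widget labels it "Computer [F]".
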(event Custom|InteractOnServer
  (Variables|Default|SetInteractToggle (not (Variables|Default|GetInteractToggle))))

(event EventBeginPlay
  (Development|ExecuteConsoleCommand "ENABLEALLSCREENMESSAGES" 0)
  (bind _asbp_interaction_area (Utilities|Casting|CastToBP_InteractionArea (Variables|/Script/Engine.ChildActorComponent|GetChildActor (Variables|Default|GetChildActor))))
  (Variables|/Game/Interaction/InteractionArea/BP_InteractionArea.BP_InteractionArea_C|SetObjectID _asbp_interaction_area (Variables|Default|GetObjectID))
  (bind _returnvalue (UserInterface|CreateWidget "/Game/FirstPerson/UI/W_Shop.W_Shop_C"))
  (bind _output_get (Variables|Default|SetShop%20UI _returnvalue))
  (UserInterface|Viewport|AddtoViewport _output_get 0)
  (CallFunction|AddPatients))

(event Collision|EventActorBeginOverlap
  (params (OtherActor :type Actor%20Object%20Reference)))

(event EventTick
  (params (DeltaSeconds :type Float%20%28single-precision%29)))

(event EventInterfaceToggleFocus
  (params (Focus :type Boolean))
  (Rendering|SetRenderCustomDepth (Variables|Default|GetCube) Focus))

(event EventInterfaceInteract
  (CallFunction|InteractonServer))

(fn ConstructionScript)

(fn OnRepInteractToggle
  (bind _returnvalue (Game|GetPlayerController 0))
  (bind _pointlight (Variables|Default|GetPointLight))
  (bind _shop_ui (Variables|Default|GetShop%20UI))
  (if (Variables|Default|GetInteractToggle)
    (bind _asbp_first_person_game_mode (Utilities|Casting|CastToBP_FirstPersonGameMode (Game|GetGameMode)))
    (if (Variables|/Game/FirstPerson/Blueprints/BP_FirstPersonGameMode.BP_FirstPersonGameMode_C|GetTutorialMode _asbp_first_person_game_mode)
      (Widget|SetVisibility (Variables|/Game/FirstPerson/Blueprints/BP_FirstPersonGameMode.BP_FirstPersonGameMode_C|GetTextBox _asbp_first_person_game_mode) "Hidden")
      (Variables|/Game/FirstPerson/Blueprints/BP_FirstPersonGameMode.BP_FirstPersonGameMode_C|SetStep _asbp_first_person_game_mode 3)
      (Rendering|SetVisibility _pointlight true false)
      (bind _outactors (Actor|GetAllActorsOfClass "/Game/FirstPerson/Blueprints/BP_FirstPersonCharacter.BP_FirstPersonCharacter_C"))
      (Variables|/Game/FirstPerson/Blueprints/BP_FirstPersonCharacter.BP_FirstPersonCharacter_C|SetCanMove (Utilities|Array|Get(acopy) _outactors) false)
      (Variables|/Script/Engine.PlayerController|SetbShowMouseCursor _returnvalue true)
      (Widget|SetVisibility _shop_ui "Visible")
      (bind _returnvalue_2 (Audio|SpawnSound2D "/Game/Assets/Audio/old-pc-monitor-switch-on-and-degaussing-8576.old-pc-monitor-switch-on-and-degaussing-8576" 1.0 1.0 0.0 0))
      (bind _output_get (Variables|Default|SetSound _returnvalue_2))
      (Audio|Components|Audio|StopDelayed _output_get 1.0))
    (else
      (Rendering|SetVisibility _pointlight false false)
      (bind _outactors_2 (Actor|GetAllActorsOfClass "/Game/FirstPerson/Blueprints/BP_FirstPersonCharacter.BP_FirstPersonCharacter_C"))
      (Variables|/Game/FirstPerson/Blueprints/BP_FirstPersonCharacter.BP_FirstPersonCharacter_C|SetCanMove (Utilities|Array|Get(acopy) _outactors_2) true)
      (Variables|/Script/Engine.PlayerController|SetbShowMouseCursor _returnvalue false)
      (Widget|SetVisibility _shop_ui "Hidden"))))

(fn AddPatients
  (for _index (range 0 (Math|Random|RandomIntegerinRange 3 5))
    (Default|AddPatienttoList (Variables|Default|GetShop%20UI))))

(fn RemovePatients
  (Default|ClearPatientList (Variables|Default|GetShop%20UI)))

(fn KeyPressOff
  (bind _returnvalue (Game|GetPlayerController 0))
  (bind _pointlight (Variables|Default|GetPointLight))
  (bind _shop_ui (Variables|Default|GetShop%20UI))
  (bind _output_get (Variables|Default|SetInteractToggle false))
  (if _output_get
    (Rendering|SetVisibility _pointlight true false)
    (bind _outactors (Actor|GetAllActorsOfClass "/Game/FirstPerson/Blueprints/BP_FirstPersonCharacter.BP_FirstPersonCharacter_C"))
    (Variables|/Game/FirstPerson/Blueprints/BP_FirstPersonCharacter.BP_FirstPersonCharacter_C|SetCanMove (Utilities|Array|Get(acopy) _outactors) false)
    (Variables|/Script/Engine.PlayerController|SetbShowMouseCursor _returnvalue true)
    (Widget|SetVisibility _shop_ui "Visible")
    (else
      (Rendering|SetVisibility _pointlight false false)
      (bind _outactors_2 (Actor|GetAllActorsOfClass "/Game/FirstPerson/Blueprints/BP_FirstPersonCharacter.BP_FirstPersonCharacter_C"))
      (Variables|/Game/FirstPerson/Blueprints/BP_FirstPersonCharacter.BP_FirstPersonCharacter_C|SetCanMove (Utilities|Array|Get(acopy) _outactors_2) true)
      (Variables|/Script/Engine.PlayerController|SetbShowMouseCursor _returnvalue false)
      (Widget|SetVisibility _shop_ui "Hidden"))))

(fn GetInteractionWidgetRef
  (bind _aswb_interaction (Utilities|Casting|CastToWB_Interaction (UserInterface|GetWidget (Variables|Default|GetWidget))))
  (Variables|/Game/Interaction/WB_Interaction.WB_Interaction_C|SetText _aswb_interaction (Utilities|String|MakeLiteralString "Computer [F]"))
  (return (Variables|Default|GetWidget)))