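; BP_Door1 is an interactable door that starts the game, labelled with a "Start Game [F]" widget and highlighted through custom depth on focus.
; BeginPlay passes its ObjectID to a child interaction area; the widget is offered only while the first character found isn't holding.
; Interaction flips InteractToggle via InteractOnServer; its OnRep sets the game mode's Begin flag, opens FirstPersonMap and calls StartGame.
; ToggleInteractable is an empty stub.
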(event Custom|InteractOnServer
  (Variables|Default|SetInteractToggle (not (Variables|Default|GetInteractToggle))))

(event EventBeginPlay
  (Development|ExecuteConsoleCommand "ENABLEALLSCREENMESSAGES" 0)
  (bind _asbp_interaction_area (Utilities|Casting|CastToBP_InteractionArea (Variables|/Script/Engine.ChildActorComponent|GetChildActor (Variables|Default|GetChildActor))))
  (Variables|/Game/Interaction/InteractionArea/BP_InteractionArea.BP_InteractionArea_C|SetObjectID _asbp_interaction_area (Variables|Default|GetObjectID))
  (CallFunction|ToggleInteractable false)
  (bind _aswb_interaction (Utilities|Casting|CastToWB_Interaction (UserInterface|GetWidget (Variables|Default|GetWidget))))
  (Variables|/Game/Interaction/WB_Interaction.WB_Interaction_C|SetText _aswb_interaction (Utilities|String|MakeLiteralString "Start Game [F]")))

(event Collision|EventActorBeginOverlap
  (params (OtherActor :type Actor%20Object%20Reference)))

(event EventInterfaceToggleFocus
  (params (Focus :type Boolean))
  (Rendering|SetRenderCustomDepth (Variables|Default|GetCube) Focus))

(event EventInterfaceInteract
  (CallFunction|InteractonServer))

(fn ConstructionScript)

(fn OnRepInteractToggle
  (bind _asbp_first_person_game_mode (Utilities|Casting|CastToBP_FirstPersonGameMode (Game|GetGameMode)))
  (Variables|/Game/FirstPerson/Blueprints/BP_FirstPersonGameMode.BP_FirstPersonGameMode_C|SetBegin _asbp_first_person_game_mode true)
  (Game|OpenLevel(byObjectReference) "/Game/FirstPerson/Maps/FirstPersonMap.FirstPersonMap")
  (Default|StartGame _asbp_first_person_game_mode))

(fn ToggleInteractable
  (params (Toggle :type Boolean)))

(fn GetInteractionWidgetRef
  (bind _outactors (Actor|GetAllActorsOfClass "/Game/FirstPerson/Blueprints/BP_FirstPersonCharacter.BP_FirstPersonCharacter_C"))
  (if (not (Variables|/Game/FirstPerson/Blueprints/BP_FirstPersonCharacter.BP_FirstPersonCharacter_C|GetIsHolding (Utilities|Array|Get(acopy) _outactors)))
    (return (Variables|Default|GetWidget))))