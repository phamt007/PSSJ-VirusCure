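; BP_FlaskTray is an interactable tray that accepts interaction only while the first-person character is holding something.
; Tick polls the first character found and switches the child BP_InteractionArea's box collision to match IsHolding.
; Focus toggles the cube's custom depth for highlighting.
; Interact calls InteractOnServer to flip InteractToggle, whose OnRep clears that character's IsHolding.
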(event Custom|InteractOnServer
  (Variables|Default|SetInteractToggle (not (Variables|Default|GetInteractToggle))))

(event EventBeginPlay
  (Development|ExecuteConsoleCommand "ENABLEALLSCREENMESSAGES" 0)
  (bind _asbp_interaction_area (Utilities|Casting|CastToBP_InteractionArea (Variables|/Script/Engine.ChildActorComponent|GetChildActor (Variables|Default|GetChildActor))))
  (Variables|/Game/Interaction/InteractionArea/BP_InteractionArea.BP_InteractionArea_C|SetObjectID _asbp_interaction_area (Variables|Default|GetObjectID)))

(event Collision|EventActorBeginOverlap
  (params (OtherActor :type Actor%20Object%20Reference)))

(event EventTick
  (params (DeltaSeconds :type Float%20%28single-precision%29))
  (bind _outactors (Actor|GetAllActorsOfClass "/Game/FirstPerson/Blueprints/BP_FirstPersonCharacter.BP_FirstPersonCharacter_C"))
  (if (Variables|/Game/FirstPerson/Blueprints/BP_FirstPersonCharacter.BP_FirstPersonCharacter_C|GetIsHolding (Utilities|Array|Get(acopy) _outactors))
    (if (not (Variables|Default|GetisActive))
      (bind _asbp_interaction_area (Utilities|Casting|CastToBP_InteractionArea (Variables|/Script/Engine.ChildActorComponent|GetChildActor (Variables|Default|GetChildActor))))
      (Collision|SetCollisionEnabled (Variables|/Game/Interaction/InteractionArea/BP_InteractionArea.BP_InteractionArea_C|GetBox _asbp_interaction_area) "QueryOnly")
      (Variables|Default|SetisActive true))
    (elif (Variables|Default|GetisActive)
      (bind _asbp_interaction_area_2 (Utilities|Casting|CastToBP_InteractionArea (Variables|/Script/Engine.ChildActorComponent|GetChildActor (Variables|Default|GetChildActor))))
      (Collision|SetCollisionEnabled (Variables|/Game/Interaction/InteractionArea/BP_InteractionArea.BP_InteractionArea_C|GetBox _asbp_interaction_area_2) "NoCollision")
      (Variables|Default|SetisActive false))))

(event EventInterfaceToggleFocus
  (params (Focus :type Boolean))
  (Rendering|SetRenderCustomDepth (Variables|Default|GetCube) Focus))

(event EventInterfaceInteract
  (CallFunction|InteractonServer))

(fn ConstructionScript)

(fn OnRepInteractToggle
  (bind _outactors (Actor|GetAllActorsOfClass "/Game/FirstPerson/Blueprints/BP_FirstPersonCharacter.BP_FirstPersonCharacter_C"))
  (Variables|/Game/FirstPerson/Blueprints/BP_FirstPersonCharacter.BP_FirstPersonCharacter_C|SetIsHolding (Utilities|Array|Get(acopy) _outactors) false))

(fn GetInteractionWidgetRef
  (return (Variables|Default|GetWidget)))