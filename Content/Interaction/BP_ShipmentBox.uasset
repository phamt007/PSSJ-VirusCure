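; BP_ShipmentBox is an interactable shipment box for vaccines that starts disabled, with a focus outline and "Shipment Box" prompt.
; ToggleInteractable switches collision on the box and its child interaction area.
; Interacting flips InteractToggle through InteractOnServer; its OnRep clears HoldingVaccine, copies the Vaccine, swaps the held item mesh and disables the box.
; Character lookups take the first BP_FirstPersonCharacter found, including the prompt's IsHolding check, rather than the interacting player.
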(event Custom|InteractOnServer
  (Variables|Default|SetInteractToggle (not (Variables|Default|GetInteractToggle))))

(event EventBeginPlay
  (Development|ExecuteConsoleCommand "ENABLEALLSCREENMESSAGES" 0)
  (bind _asbp_interaction_area (Utilities|Casting|CastToBP_InteractionArea (Variables|/Script/Engine.ChildActorComponent|GetChildActor (Variables|Default|GetChildActor))))
  (Variables|/Game/Interaction/InteractionArea/BP_InteractionArea.BP_InteractionArea_C|SetObjectID _asbp_interaction_area (Variables|Default|GetObjectID))
  (CallFunction|ToggleInteractable false)
  (bind _aswb_interaction (Utilities|Casting|CastToWB_Interaction (UserInterface|GetWidget (Variables|Default|GetWidget))))
  (Variables|/Game/Interaction/WB_Interaction.WB_Interaction_C|SetText _aswb_interaction (Utilities|String|MakeLiteralString "Shipment Box")))

(event Collision|EventActorBeginOverlap
  (params (OtherActor :type Actor%20Object%20Reference)))

(event EventInterfaceToggleFocus
  (params (Focus :type Boolean))
  (Rendering|SetRenderCustomDepth (Variables|Default|GetCube) Focus))

(event EventInterfaceInteract
  (CallFunction|InteractonServer))

(fn ConstructionScript)

(fn OnRepInteractToggle
  (bind _outactors (Actor|GetAllActorsOfClass "/Game/FirstPerson/Blueprints/BP_FirstPersonCharacter.BP_FirstPersonCharacter_C"))
  (Variables|/Game/FirstPerson/Blueprints/BP_FirstPersonCharacter.BP_FirstPersonCharacter_C|SetHoldingVaccine (Utilities|Array|Get(acopy) _outactors) false)
  (Variables|Default|SetVaccine (Variables|/Game/FirstPerson/Blueprints/BP_FirstPersonCharacter.BP_FirstPersonCharacter_C|GetVaccine (Utilities|Array|Get(acopy) _outactors)))
  (CallFunction|ToggleInteractable false)
  (Components|StaticMesh|SetStaticMesh (Variables|/Game/FirstPerson/Blueprints/BP_FirstPersonCharacter.BP_FirstPersonCharacter_C|GetItem (Utilities|Array|Get(acopy) _outactors)) (Variables|Default|GetMesh)))

(fn ToggleInteractable
  (params (Toggle :type Boolean))
  (if Toggle
    (Development|PrintString "Can ship")
    (bind _asbp_interaction_area (Utilities|Casting|CastToBP_InteractionArea (Variables|/Script/Engine.ChildActorComponent|GetChildActor (Variables|Default|GetChildActor))))
    (Collision|SetCollisionEnabled (Variables|/Game/Interaction/InteractionArea/BP_InteractionArea.BP_InteractionArea_C|GetBox _asbp_interaction_area) "QueryOnly")
    (Collision|SetCollisionEnabled (Variables|Default|GetCube) "QueryAndProbe")
    (else
      (Development|PrintString "Cant ship")
      (bind _asbp_interaction_area_2 (Utilities|Casting|CastToBP_InteractionArea (Variables|/Script/Engine.ChildActorComponent|GetChildActor (Variables|Default|GetChildActor))))
      (Collision|SetCollisionEnabled (Variables|/Game/Interaction/InteractionArea/BP_InteractionArea.BP_InteractionArea_C|GetBox _asbp_interaction_area_2) "NoCollision")
      (Collision|SetCollisionEnabled (Variables|Default|GetCube) "NoCollision"))))

(fn GetInteractionWidgetRef
  (bind _outactors (Actor|GetAllActorsOfClass "/Game/FirstPerson/Blueprints/BP_FirstPersonCharacter.BP_FirstPersonCharacter_C"))
  (if (not (Variables|/Game/FirstPerson/Blueprints/BP_FirstPersonCharacter.BP_FirstPersonCharacter_C|GetIsHolding (Utilities|Array|Get(acopy) _outactors)))
    (return (Variables|Default|GetWidget))))