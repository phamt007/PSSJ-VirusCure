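; BP_VirusContainer holds the active virus, picked at random from a Viruses list, and supplies random symptoms for it.
; GenerateRandomVirus rebuilds PotentialSymptoms as a weighted bag, adding each of the virus's four symptom names more often the higher its severity.
; GenerateRandomSymptom draws uniformly from that bag, so severe symptoms come up more often than moderate or mild ones.
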(event EventBeginPlay)

(event Collision|EventActorBeginOverlap
  (params (OtherActor :type Actor%20Object%20Reference)))

(event EventTick
  (params (DeltaSeconds :type Float%20%28single-precision%29)))

(fn ConstructionScript)

(fn GenerateRandomVirus
  (bind _viruses (Variables|Default|GetViruses))
  (Variables|Default|SetCurrentVirus "")
  (Utilities|Array|Clear (Variables|Default|GetPotentialSymptoms))
  (Variables|Default|SetCurrentVirus (Utilities|Array|Get(acopy) _viruses (Math|Random|RandomIntegerinRange 0 (- (Utilities|Array|Length _viruses) 1))))
  (switch Utilities|FlowControl|Switch|SwitchonSeverity (.Severity (Utilities|Struct|BreakSymptom (.Symptom1 (Utilities|Struct|BreakVirus (Variables|Default|GetCurrentVirus)))))
    (:NewEnumerator0
      (for _index (range 0 0)
        (Utilities|Array|Add (Variables|Default|GetPotentialSymptoms) (.Name (Utilities|Struct|BreakSymptom (.Symptom1 (Utilities|Struct|BreakVirus (Variables|Default|GetCurrentVirus))))))))
    (:NewEnumerator1
      (for _index_2 (range 0 2)
        (Utilities|Array|Add (Variables|Default|GetPotentialSymptoms) (.Name (Utilities|Struct|BreakSymptom (.Symptom1 (Utilities|Struct|BreakVirus (Variables|Default|GetCurrentVirus))))))))
    (:NewEnumerator2
      (for _index_3 (range 0 4)
        (Utilities|Array|Add (Variables|Default|GetPotentialSymptoms) (.Name (Utilities|Struct|BreakSymptom (.Symptom1 (Utilities|Struct|BreakVirus (Variables|Default|GetCurrentVirus)))))))))
  (switch Utilities|FlowControl|Switch|SwitchonSeverity (.Severity (Utilities|Struct|BreakSymptom (.Symptom2 (Utilities|Struct|BreakVirus (Variables|Default|GetCurrentVirus)))))
    (:NewEnumerator0
      (for _index_4 (range 0 0)
        (Utilities|Array|Add (Variables|Default|GetPotentialSymptoms) (.Name (Utilities|Struct|BreakSymptom (.Symptom2 (Utilities|Struct|BreakVirus (Variables|Default|GetCurrentVirus))))))))
    (:NewEnumerator1
      (for _index_5 (range 0 2)
        (Utilities|Array|Add (Variables|Default|GetPotentialSymptoms) (.Name (Utilities|Struct|BreakSymptom (.Symptom2 (Utilities|Struct|BreakVirus (Variables|Default|GetCurrentVirus))))))))
    (:NewEnumerator2
      (for _index_6 (range 0 4)
        (Utilities|Array|Add (Variables|Default|GetPotentialSymptoms) (.Name (Utilities|Struct|BreakSymptom (.Symptom2 (Utilities|Struct|BreakVirus (Variables|Default|GetCurrentVirus)))))))))
  (switch Utilities|FlowControl|Switch|SwitchonSeverity (.Severity (Utilities|Struct|BreakSymptom (.Symptom3 (Utilities|Struct|BreakVirus (Variables|Default|GetCurrentVirus)))))
    (:NewEnumerator0
      (for _index_7 (range 0 0)
        (Utilities|Array|Add (Variables|Default|GetPotentialSymptoms) (.Name (Utilities|Struct|BreakSymptom (.Symptom3 (Utilities|Struct|BreakVirus (Variables|Default|GetCurrentVirus))))))))
    (:NewEnumerator1
      (for _index_8 (range 0 2)
        (Utilities|Array|Add (Variables|Default|GetPotentialSymptoms) (.Name (Utilities|Struct|BreakSymptom (.Symptom3 (Utilities|Struct|BreakVirus (Variables|Default|GetCurrentVirus))))))))
    (:NewEnumerator2
      (for _index_9 (range 0 4)
        (Utilities|Array|Add (Variables|Default|GetPotentialSymptoms) (.Name (Utilities|Struct|BreakSymptom (.Symptom3 (Utilities|Struct|BreakVirus (Variables|Default|GetCurrentVirus)))))))))
  (switch Utilities|FlowControl|Switch|SwitchonSeverity (.Severity (Utilities|Struct|BreakSymptom (.Symptom4 (Utilities|Struct|BreakVirus (Variables|Default|GetCurrentVirus)))))
    (:NewEnumerator0
      (for _index_10 (range 0 0)
        (Utilities|Array|Add (Variables|Default|GetPotentialSymptoms) (.Name (Utilities|Struct|BreakSymptom (.Symptom4 (Utilities|Struct|BreakVirus (Variables|Default|GetCurrentVirus))))))))
    (:NewEnumerator1
      (for _index_11 (range 0 2)
        (Utilities|Array|Add (Variables|Default|GetPotentialSymptoms) (.Name (Utilities|Struct|BreakSymptom (.Symptom4 (Utilities|Struct|BreakVirus (Variables|Default|GetCurrentVirus))))))))
    (:NewEnumerator2
      (for _index_12 (range 0 4)
        (Utilities|Array|Add (Variables|Default|GetPotentialSymptoms) (.Name (Utilities|Struct|BreakSymptom (.Symptom4 (Utilities|Struct|BreakVirus (Variables|Default|GetCurrentVirus))))))))))

(fn GenerateRandomSymptom
  (bind _potentialsymptoms (Variables|Default|GetPotentialSymptoms))
  (return (Utilities|Array|Get(acopy) _potentialsymptoms (Math|Random|RandomIntegerinRange 0 (- (Utilities|Array|Length _potentialsymptoms) 1)))))