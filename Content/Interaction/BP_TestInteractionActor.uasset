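; Test interactable actor that highlights its cube through custom depth on focus and passes its ObjectID to a child BP_InteractionArea.
; Interacting calls InteractOnServer to flip InteractToggle, whose OnRep switches the point light, movement lock and mouse cursor.
; Its widget getter returns the widget only while the character is not holding.
; Character lookups take the first BP_FirstPersonCharacter found, and the cursor change targets player controller 0.
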(event Custom|InteractOnServer
  (Variables|Default|SetInteractToggle (not (Variables|Default|GetInteractToggle))))

(event EventBeginPlay
  (Development|ExecuteConsoleCommand "ENABLEALLSCREENMESSAGES" 0)
  (bind _asbp_interaction_area (Utilities|Casting|CastToBP_InteractionArea (Variables|/Script/Engine.ChildActorComponent|GetChildActor (Variables|Default|GetChildActor))))
  (Variables|/Game/Interaction/InteractionArea/BP_InteractionArea.BP_InteractionArea_C|SetObjectID _asbp_interaction_area (Variables|Default|GetObjectID)))

(event Collision|EventActorBeginOverlap
  (params (OtherActor :type Actor%20Object%20Reference)))

(event EventTick
  (params (DeltaSeconds :type Float%20%28single-precision%29)))

(event EventInterfaceToggleFocus
  (params (Focus :type Boolean))
  (Rendering|SetRenderCustomDepth (Variables|Default|GetCube) Focus))

(event EventInterfaceInteract
  (CallFunction|InteractonServer))

(fn ConstructionScript)

(fn OnRepInteractToggle
  (bind _returnvalue (Game|GetPlayerController 0))
  (bind _pointlight (Variables|Default|GetPointLight))
  (if (Variables|Default|GetInteractToggle)
    (Rendering|SetVisibility _pointlight true false)
    (bind _outactors (Actor|GetAllActorsOfClass "/Game/FirstPerson/Blueprints/BP_FirstPersonCharacter.BP_FirstPersonCharacter_C"))
    (Variables|/Game/FirstPerson/Blueprints/BP_FirstPersonCharacter.BP_FirstPersonCharacter_C|SetCanMove (Utilities|Array|Get(acopy) _outactors) false)
    (Variables|/Script/Engine.PlayerController|SetbShowMouseCursor _returnvalue true)
    (else
      (Rendering|SetVisibility _pointlight false false)
      (bind _outactors_2 (Actor|GetAllActorsOfClass "/Game/FirstPerson/Blueprints/BP_FirstPersonCharacter.BP_FirstPersonCharacter_C"))
      (Variables|/Game/FirstPerson/Blueprints/BP_FirstPersonCharacter.BP_FirstPersonCharacter_C|SetCanMove (Utilities|Array|Get(acopy) _outactors_2) true)
      (Variables|/Script/Engine.PlayerController|SetbShowMouseCursor _returnvalue false))))

(fn GetInteractionWidgetRef
  (bind _outactors (Actor|GetAllActorsOfClass "/Game/FirstPerson/Blueprints/BP_FirstPersonCharacter.BP_FirstPersonCharacter_C"))
  (if (not (Variables|/Game/FirstPerson/Blueprints/BP_FirstPersonCharacter.BP_FirstPersonCharacter_C|GetIsHolding (Utilities|Array|Get(acopy) _outactors)))
    (return (Variables|Default|GetWidget))))