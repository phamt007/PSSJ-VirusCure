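; Interactable door that advances the game, prompting "Go Next Month [F]" and highlighting its cube via custom depth on focus.
; BeginPlay passes its ObjectID to a child interaction area, sets up the prompt widget and calls StartGame on the game mode.
; Interacting flips InteractToggle through InteractOnServer; its OnRep calls the game mode's Timer and plays a door sound.
; The prompt widget is returned only when the first found player character holds nothing.
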(event Custom|InteractOnServer
  (Variables|Default|SetInteractToggle (not (Variables|Default|GetInteractToggle))))

(event EventBeginPlay
  (Development|ExecuteConsoleCommand "ENABLEALLSCREENMESSAGES" 0)
  (bind _asbp_interaction_area (Utilities|Casting|CastToBP_InteractionArea (Variables|/Script/Engine.ChildActorComponent|GetChildActor (Variables|Default|GetChildActor))))
  (Variables|/Game/Interaction/InteractionArea/BP_InteractionArea.BP_InteractionArea_C|SetObjectID _asbp_interaction_area (Variables|Default|GetObjectID))
  (CallFunction|ToggleInteractable false)
  (bind _aswb_interaction (Utilities|Casting|CastToWB_Interaction (UserInterface|GetWidget (Variables|Default|GetWidget))))
  (Variables|/Game/Interaction/WB_Interaction.WB_Interaction_C|SetText _aswb_interaction (Utilities|String|MakeLiteralString "Go Next Month [F]"))
  (Development|PrintString "look")
  (Default|EditSizeBox _aswb_interaction 4e+02)
  (bind _asbp_first_person_game_mode (Utilities|Casting|CastToBP_FirstPersonGameMode (Game|GetGameMode)))
  (Default|StartGame _asbp_first_person_game_mode))

(event Collision|EventActorBeginOverlap
  (params (OtherActor :type Actor%20Object%20Reference)))

(event EventInterfaceToggleFocus
  (params (Focus :type Boolean))
  (Rendering|SetRenderCustomDepth (Variables|Default|GetCube) Focus))

(event EventInterfaceInteract
  (CallFunction|InteractonServer))

(fn ConstructionScript)

(fn OnRepInteractToggle
  (bind _asbp_first_person_game_mode (Utilities|Casting|CastToBP_FirstPersonGameMode (Game|GetGameMode)))
  (Default|Timer _asbp_first_person_game_mode)
  (bind _returnvalue (Audio|SpawnSound2D "/Game/Assets/Audio/door-open-close-45475.door-open-close-45475" 1.0 1.0 0.0 0))
  (Variables|Default|SetSound _returnvalue))

(fn ToggleInteractable
  (params (Toggle :type Boolean)))

(fn GetInteractionWidgetRef
  (bind _outactors (Actor|GetAllActorsOfClass "/Game/FirstPerson/Blueprints/BP_FirstPersonCharacter.BP_FirstPersonCharacter_C"))
  (if (not (Variables|/Game/FirstPerson/Blueprints/BP_FirstPersonCharacter.BP_FirstPersonCharacter_C|GetIsHolding (Utilities|Array|Get(acopy) _outactors)))
    (return (Variables|Default|GetWidget))))