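; Interactable button that triggers mixing on the first BP_Mixer found in the level.
; Passes its ObjectID to a child interaction area, highlights its cube via custom depth on focus, and supplies a "Mix Ingredient" prompt widget.
; Interaction toggles a replicated flag through InteractOnServer; its OnRep advances the tutorial timer in tutorial mode, then calls Mix.
; The OnRep requires the GameMode cast to succeed, so Mix effectively runs only on the server.
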(event Custom|InteractOnServer
  (Variables|Default|SetInteractToggle (not (Variables|Default|GetInteractToggle))))

(event EventBeginPlay
  (Development|ExecuteConsoleCommand "ENABLEALLSCREENMESSAGES" 0)
  (bind _asbp_interaction_area (Utilities|Casting|CastToBP_InteractionArea (Variables|/Script/Engine.ChildActorComponent|GetChildActor (Variables|Default|GetChildActor))))
  (Variables|/Game/Interaction/InteractionArea/BP_InteractionArea.BP_InteractionArea_C|SetObjectID _asbp_interaction_area (Variables|Default|GetObjectID)))

(event Collision|EventActorBeginOverlap
  (params (OtherActor :type Actor%20Object%20Reference)))

(event EventTick
  (params (DeltaSeconds :type Float%20%28single-precision%29)))

(event EventInterfaceToggleFocus
  (params (Focus :type Boolean))
  (Rendering|SetRenderCustomDepth (Variables|Default|GetCube) Focus))

(event EventInterfaceInteract
  (CallFunction|InteractonServer))

(fn ConstructionScript)

(fn OnRepInteractToggle
  (bind _asbp_first_person_game_mode (Utilities|Casting|CastToBP_FirstPersonGameMode (Game|GetGameMode)))
  (if (Variables|/Game/FirstPerson/Blueprints/BP_FirstPersonGameMode.BP_FirstPersonGameMode_C|GetTutorialMode _asbp_first_person_game_mode)
    (Default|TutorialTimer _asbp_first_person_game_mode 1.0))
  (bind _outactors (Actor|GetAllActorsOfClass "/Game/Interaction/BP_Mixer.BP_Mixer_C"))
  (Default|Mix (Utilities|Array|Get(acopy) _outactors)))

(fn GetInteractionWidgetRef
  (bind _aswb_interaction (Utilities|Casting|CastToWB_Interaction (UserInterface|GetWidget (Variables|Default|GetWidget))))
  (Variables|/Game/Interaction/WB_Interaction.WB_Interaction_C|SetText _aswb_interaction (Utilities|String|MakeLiteralString "Mix Ingredient [F]"))
  (Default|EditSizeBox _aswb_interaction 4e+02)
  (return (Variables|Default|GetWidget)))