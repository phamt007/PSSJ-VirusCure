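; BP_TrayInteractionArea is a tray interaction area that relays focus changes to its parent actor.
; Its ToggleFocus event stores the focus state, passes it to the parent through a message call and gets the parent's interaction widget.
; It shows or hides that widget with focus only while the first BP_FirstPersonCharacter found by GetAllActorsOfClass is not holding, otherwise leaving its visibility unchanged.
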(event Custom|ToggleFocus
  (params (Focused :type Boolean))
  (Variables|Default|SetFocused Focused)
  (Class|BIInteraction|InterfaceToggleFocus(Message) (Actor|GetParentActor) (Variables|Default|GetFocused))
  (bind _ref (Class|BIInteraction|GetInteractionWidgetRef(Message) (Actor|GetParentActor)))
  (bind _outactors (Actor|GetAllActorsOfClass "/Game/FirstPerson/Blueprints/BP_FirstPersonCharacter.BP_FirstPersonCharacter_C"))
  (if (not (Variables|/Game/FirstPerson/Blueprints/BP_FirstPersonCharacter.BP_FirstPersonCharacter_C|GetIsHolding (Utilities|Array|Get(acopy) _outactors)))
    (Development|SetHiddeninGame _ref (not (Variables|Default|GetFocused)) false)))

(fn ConstructionScript)