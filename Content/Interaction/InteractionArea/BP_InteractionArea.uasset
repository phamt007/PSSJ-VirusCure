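; Interaction area actor that relays focus changes to its parent interactable, such as flasks, trays, cubes, mixer, shipment box or door.
; ToggleFocus switches on ObjectID, shows or hides the parent's interaction widget and forwards focus through interface messages.
; Flasks check the first-person character's matching ingredient quantity, withholding focus and blocking CanInteract when empty, then restoring CanInteract on unfocus.
; DisableHighlight reapplies the stored Focused state to the widget and parent.
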(event Custom|ToggleFocus
  (params (Focused :type Boolean))
  (Variables|Default|SetFocused Focused)
  (switch int (Variables|Default|GetObjectID)
    (:1
      ;[1 1 1] FlaskTray
      (Class|BIInteraction|InterfaceToggleFocus(Message) (Actor|GetParentActor) (Variables|Default|GetFocused))
      (bind _ref (Class|BIInteraction|GetInteractionWidgetRef(Message) (Actor|GetParentActor)))
      (Development|SetHiddeninGame _ref (not (Variables|Default|GetFocused)) false))
    (:2
      ;[1 1 1] Flask
      (bind _ref_2 (Class|BIInteraction|GetInteractionWidgetRef(Message) (Actor|GetParentActor)))
      (Development|SetHiddeninGame _ref_2 (not (Variables|Default|GetFocused)) false)
      (if (Variables|Default|GetFocused)
        (bind _outactors (Actor|GetAllActorsOfClass "/Game/FirstPerson/Blueprints/BP_FirstPersonCharacter.BP_FirstPersonCharacter_C"))
        (bind _asbp_flask (Utilities|Casting|CastToBP_Flask (Actor|GetParentActor)))
        (bind _ingredient (Default|GetIngredient (Utilities|Array|Get(acopy) _outactors) (Variables|/Game/Interaction/BP_Flask.BP_Flask_C|GetFlaskText _asbp_flask)))
        (if (> (.Quantity (Utilities|Struct|BreakIngredient _ingredient)) 0)
          (Class|BIInteraction|InterfaceToggleFocus(Message) (Actor|GetParentActor) (Variables|Default|GetFocused))
          (else
            (bind _outactors_2 (Actor|GetAllActorsOfClass "/Game/FirstPerson/Blueprints/BP_FirstPersonCharacter.BP_FirstPersonCharacter_C"))
            (Variables|/Game/FirstPerson/Blueprints/BP_FirstPersonCharacter.BP_FirstPersonCharacter_C|SetCanInteract (Utilities|Array|Get(acopy) _outactors_2) false)))
        (else
          (Class|BIInteraction|InterfaceToggleFocus(Message) (Actor|GetParentActor) (Variables|Default|GetFocused))
          (bind _outactors_3 (Actor|GetAllActorsOfClass "/Game/FirstPerson/Blueprints/BP_FirstPersonCharacter.BP_FirstPersonCharacter_C"))
          (Variables|/Game/FirstPerson/Blueprints/BP_FirstPersonCharacter.BP_FirstPersonCharacter_C|SetCanInteract (Utilities|Array|Get(acopy) _outactors_3) true))))
    (:3
      ;[1 1 1] Cube
      (Class|BIInteraction|InterfaceToggleFocus(Message) (Actor|GetParentActor) (Variables|Default|GetFocused))
      (bind _ref_3 (Class|BIInteraction|GetInteractionWidgetRef(Message) (Actor|GetParentActor)))
      (Development|SetHiddeninGame _ref_3 (not (Variables|Default|GetFocused)) false))
    (:4
      ;[1 1 1] Mixer
      (Class|BIInteraction|InterfaceToggleFocus(Message) (Actor|GetParentActor) (Variables|Default|GetFocused))
      (bind _ref_4 (Class|BIInteraction|GetInteractionWidgetRef(Message) (Actor|GetParentActor)))
      (Development|SetHiddeninGame _ref_4 (not (Variables|Default|GetFocused)) false))
    (:5
      ;[1 1 1] MixerButton
      (Class|BIInteraction|InterfaceToggleFocus(Message) (Actor|GetParentActor) (Variables|Default|GetFocused))
      (bind _ref_5 (Class|BIInteraction|GetInteractionWidgetRef(Message) (Actor|GetParentActor)))
      (Development|SetHiddeninGame _ref_5 (not (Variables|Default|GetFocused)) false))
    (:6
      ;[1 1 1] ShipmentBox
      (Class|BIInteraction|InterfaceToggleFocus(Message) (Actor|GetParentActor) (Variables|Default|GetFocused))
      (bind _ref_6 (Class|BIInteraction|GetInteractionWidgetRef(Message) (Actor|GetParentActor)))
      (Development|SetHiddeninGame _ref_6 (not (Variables|Default|GetFocused)) false))
    (:7
      ;[1 1 1] Door
      (Class|BIInteraction|InterfaceToggleFocus(Message) (Actor|GetParentActor) (Variables|Default|GetFocused))
      (bind _ref_7 (Class|BIInteraction|GetInteractionWidgetRef(Message) (Actor|GetParentActor)))
      (Development|SetHiddeninGame _ref_7 (not (Variables|Default|GetFocused)) false))))

(fn ConstructionScript)

(fn DisableHighlight
  (bind _ref (Class|BIInteraction|GetInteractionWidgetRef(Message) (Actor|GetParentActor)))
  (Development|SetHiddeninGame _ref (not (Variables|Default|GetFocused)) false)
  (Class|BIInteraction|InterfaceToggleFocus(Message) (Actor|GetParentActor) (Variables|Default|GetFocused)))