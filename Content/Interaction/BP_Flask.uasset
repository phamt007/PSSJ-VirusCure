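; BP_Flask is an interactable ingredient flask that puts an item in the first-person character's hand and decrements that ingredient's count.
; Interaction flips InteractToggle through InteractOnServer, and its OnRep sets the held mesh and holding state on the first character found.
; Tick switches flask and child interaction-area collision off while that character holds something.
; Focus toggles custom depth, and the widget getter displays ingredient name and quantity.
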(event Custom|InteractOnServer
  (Variables|Default|SetInteractToggle (not (Variables|Default|GetInteractToggle))))

(event EventBeginPlay
  (Development|ExecuteConsoleCommand "ENABLEALLSCREENMESSAGES" 0)
  (bind _asbp_interaction_area (Utilities|Casting|CastToBP_InteractionArea (Variables|/Script/Engine.ChildActorComponent|GetChildActor (Variables|Default|GetChildActor))))
  (Variables|/Game/Interaction/InteractionArea/BP_InteractionArea.BP_InteractionArea_C|SetObjectID _asbp_interaction_area (Variables|Default|GetObjectID)))

(event Collision|EventActorBeginOverlap
  (params (OtherActor :type Actor%20Object%20Reference)))

(event EventTick
  (params (DeltaSeconds :type Float%20%28single-precision%29))
  (bind _outactors (Actor|GetAllActorsOfClass "/Game/FirstPerson/Blueprints/BP_FirstPersonCharacter.BP_FirstPersonCharacter_C"))
  (if (Variables|/Game/FirstPerson/Blueprints/BP_FirstPersonCharacter.BP_FirstPersonCharacter_C|GetIsHolding (Utilities|Array|Get(acopy) _outactors))
    (if (Variables|Default|GetisActive)
      (bind _asbp_interaction_area (Utilities|Casting|CastToBP_InteractionArea (Variables|/Script/Engine.ChildActorComponent|GetChildActor (Variables|Default|GetChildActor))))
      (Collision|SetCollisionEnabled (Variables|/Game/Interaction/InteractionArea/BP_InteractionArea.BP_InteractionArea_C|GetBox _asbp_interaction_area) "NoCollision")
      (Collision|SetCollisionEnabled (Variables|Default|GetCube) "NoCollision")
      (Variables|Default|SetisActive false))
    (elif (not (Variables|Default|GetisActive))
      (bind _asbp_interaction_area_2 (Utilities|Casting|CastToBP_InteractionArea (Variables|/Script/Engine.ChildActorComponent|GetChildActor (Variables|Default|GetChildActor))))
      (Collision|SetCollisionEnabled (Variables|/Game/Interaction/InteractionArea/BP_InteractionArea.BP_InteractionArea_C|GetBox _asbp_interaction_area_2) "QueryOnly")
      (Collision|SetCollisionEnabled (Variables|Default|GetCube) "QueryAndProbe")
      (Variables|Default|SetisActive true))))

(event EventInterfaceToggleFocus
  (params (Focus :type Boolean))
  (Rendering|SetRenderCustomDepth (Variables|Default|GetCube) Focus))

(event EventInterfaceInteract
  (CallFunction|InteractonServer))

(fn ConstructionScript)

(fn OnRepInteractToggle
  (bind _outactors (Actor|GetAllActorsOfClass "/Game/FirstPerson/Blueprints/BP_FirstPersonCharacter.BP_FirstPersonCharacter_C"))
  (if (Variables|/Game/FirstPerson/Blueprints/BP_FirstPersonCharacter.BP_FirstPersonCharacter_C|GetCanInteract (Utilities|Array|Get(acopy) _outactors))
    (bind _outactors_2 (Actor|GetAllActorsOfClass "/Game/FirstPerson/Blueprints/BP_FirstPersonCharacter.BP_FirstPersonCharacter_C"))
    (Variables|/Game/FirstPerson/Blueprints/BP_FirstPersonCharacter.BP_FirstPersonCharacter_C|SetIsHolding (Utilities|Array|Get(acopy) _outactors_2) true)
    (bind _outactors_3 (Actor|GetAllActorsOfClass "/Game/FirstPerson/Blueprints/BP_FirstPersonCharacter.BP_FirstPersonCharacter_C"))
    (Components|StaticMesh|SetStaticMesh (Variables|/Game/FirstPerson/Blueprints/BP_FirstPersonCharacter.BP_FirstPersonCharacter_C|GetItem (Utilities|Array|Get(acopy) _outactors_3)) "/Engine/BasicShapes/Cylinder.Cylinder")
    (Default|IncrementIngredient (Utilities|Array|Get(acopy) _outactors_3) (Variables|Default|GetFlaskText) -1)))

(fn GetInteractionWidgetRef
  (bind _aswb_interaction (Utilities|Casting|CastToWB_Interaction (UserInterface|GetWidget (Variables|Default|GetWidget))))
  (bind _outactors (Actor|GetAllActorsOfClass "/Game/FirstPerson/Blueprints/BP_FirstPersonCharacter.BP_FirstPersonCharacter_C"))
  (bind _ingredient (Default|GetIngredient (Utilities|Array|Get(acopy) _outactors) (Variables|Default|GetFlaskText)))
  (Variables|/Game/Interaction/WB_Interaction.WB_Interaction_C|SetText _aswb_interaction (Utilities|String|Append (Utilities|String|Append (.Name (Utilities|Struct|BreakIngredient _ingredient)) (Utilities|String|MakeLiteralString " x")) (Utilities|String|ToString(Integer) (.Quantity (Utilities|Struct|BreakIngredient _ingredient)))))
  (return (Variables|Default|GetWidget)))